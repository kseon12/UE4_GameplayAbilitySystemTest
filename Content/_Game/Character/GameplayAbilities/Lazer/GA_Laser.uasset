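; GA_Laser is a gameplay ability that casts a channeled laser from the character.
; After committing, it plays a cast montage, then spawns BP_Laser on the mesh's LaserSocket and switches the character to camera-controlled rotation.
; Skill.Laser.DealDamage events apply damage and push targets away from the laser's end detector while cost is affordable, otherwise ending the ability.
; Ending removes mana-drain effects, destroys the laser and restores rotation.
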(event `self.K2_ActivateAbility`
  (`self.K2_CommitAbility`)
  (`self.DoUICooldown`)
  (`AbilityTask_PlayMontageAndWait.CreatePlayMontageAndWaitProxy` "None" "/Game/_Game/Character/Animation/AM_Cast_Laser.AM_Cast_Laser"
    (:`then`
      (`KismetSystemLibrary.Delay` 0.3)
      (bind _basecharacter (`self.Get Player Character and Controller`))
      (bind (_asynctaskproxy _spawnedactor) (`AbilityTask_SpawnActor.SpawnActor` (struct) "/Game/_Game/Character/GameplayAbilities/Lazer/BP_Laser.BP_Laser_C" _basecharacter)
        (:`then`
          (bind _output_get (set `self.SpawnedLaser` _spawnedactor))
          (`Actor.K2_AttachToComponent` _output_get (`Character.Mesh` _basecharacter) "LaserSocket" "SnapToTarget" "SnapToTarget" "KeepRelative" true)
          (`/Game/_Game/Character/BP_BaseCharacter.MakeCameraControlRotation` _basecharacter true)
          (bind (_asynctaskproxy_2 _payload) (`AbilityTask_WaitGameplayEvent.WaitGameplayEvent` (struct :`TagName` "Skill.Laser.DealDamage") null)
            (:`EventReceived`
              (bind _returnvalue (`self.K2_CheckAbilityCost`))
              (if _returnvalue
                (bind (_eventtag _instigator _target _optionalobject _optionalobject2 _contexthandle _instigatortags _targettags _eventmagnitude _targetdata) (break `GameplayEventData` _payload))
                (`self.BP_ApplyGameplayEffectToTarget` _targetdata "/Game/_Game/Character/GameplayAbilities/Lazer/GE_Laser_DealDamage.GE_Laser_DealDamage_C")
                (for _array_element (`AbilitySystemBlueprintLibrary.GetActorsFromTargetData` _targetdata)
                  (bind _asbp_base_character (cast `/Game/_Game/Character/BP_BaseCharacter` _array_element))
                  (`/Game/_Game/Character/BP_BaseCharacter.PushCharacter` _asbp_base_character (`KismetMathLibrary.Normal` (- (`Actor.K2_GetActorLocation` _asbp_base_character) (`SceneComponent.K2_GetComponentLocation` (`/Game/_Game/Character/GameplayAbilities/Lazer/BP_Laser.LaserEndDetector` (cast `/Game/_Game/Character/GameplayAbilities/Lazer/BP_Laser` (`self.SpawnedLaser`) :!pure true))))) 500.0 0.3))
                (else
                  (`self.K2_EndAbility`))))))))))

(event `self.K2_OnEndAbility`
  (params (bWasCancelled :type Boolean))
  (`self.BP_RemoveGameplayEffectFromOwnerWithAssetTags` (struct :`GameplayTags` (struct :`(TagName` "Skill.Laser.ManaDrain"))))
  (`Actor.K2_DestroyActor` (`self.SpawnedLaser`))
  (bind _basecharacter (`self.Get Player Character and Controller`))
  (`/Game/_Game/Character/BP_BaseCharacter.MakeCameraControlRotation` _basecharacter false))