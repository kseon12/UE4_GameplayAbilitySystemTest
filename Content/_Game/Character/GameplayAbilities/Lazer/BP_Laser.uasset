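; Laser beam actor for the laser gameplay ability that repeatedly damages hostile characters at its far end.
; Each tick it stretches the beam by setting the ABP_LaserBeam end-bone offset from the LaserEndDetector's distance minus the original mesh length.
; Detector overlaps maintain a list of characters hostile to the instigator.
; A looping timer sends that list to the instigator as target data in a Skill.Laser.DealDamage gameplay event.
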(event `self.ReceiveBeginPlay`
  (set `self.BeamOriginalLength` (`KismetMathLibrary.VSize` (- (`SceneComponent.GetSocketLocation` (`self.LaserMesh`) "End") (`self.K2_GetActorLocation`))))
  (`KismetSystemLibrary.K2_SetTimerDelegate` (delegate `SendDealDamageEffect`) 0.3 true))

(event `SendDealDamageEffect`
  ;[1 1 1] Comment
  (`AbilitySystemBlueprintLibrary.SendGameplayEventToActor` (`self.GetInstigator`) (struct :`TagName` "Skill.Laser.DealDamage") (make `GameplayEventData` (struct) null null null null (struct) (struct) (struct) 0.0 (`AbilitySystemBlueprintLibrary.AbilityTargetDataFromActorArray` (`self.OverlapingActors`)))))

(event `self.ReceiveTick`
  (params (DeltaSeconds :type "Float (single-precision)"))
  ;[1 1 1] Comment
  (bind _asabp_laser_beam (cast `/Game/_Game/Character/GameplayAbilities/Lazer/LazerAssets/ABP_LaserBeam` (`SkeletalMeshComponent.GetAnimInstance` (`self.LaserMesh`))))
  (set `/Game/_Game/Character/GameplayAbilities/Lazer/LazerAssets/ABP_LaserBeam.EndBoneOffset` (`KismetMathLibrary.MakeVector` (- (`KismetMathLibrary.VSize` (- (`SceneComponent.K2_GetComponentLocation` (`self.LaserEndDetector`)) (`self.K2_GetActorLocation`))) (`self.BeamOriginalLength`))) _asabp_laser_beam))

(event `self.LaserEndDetector.OnComponentBeginOverlap`
  (params (OverlappedComponent :type "PrimitiveComponent Object Reference") (OtherActor :type "Actor Object Reference") (OtherComp :type "PrimitiveComponent Object Reference") (OtherBodyIndex :type Integer) (bFromSweep :type Boolean) (SweepResult :type "HitResult Structure (by ref)"))
  ;[1 1 1] Comment
  (bind _asbp_base_character (cast `/Game/_Game/Character/BP_BaseCharacter` OtherActor))
  (bind _asbp_base_character_2 (cast `/Game/_Game/Character/BP_BaseCharacter` (`self.GetInstigator`)))
  (bind _returnvalue (`BaseCharacter.IsTargetHostile` _asbp_base_character_2 _asbp_base_character))
  (if _returnvalue
    (`KismetArrayLibrary.Array_AddUnique` (`self.OverlapingActors`) _asbp_base_character)))

(event `self.LaserEndDetector.OnComponentEndOverlap`
  (params (OverlappedComponent :type "PrimitiveComponent Object Reference") (OtherActor :type "Actor Object Reference") (OtherComp :type "PrimitiveComponent Object Reference") (OtherBodyIndex :type Integer))
  ;[1 1 1] Comment
  (bind _asbp_base_character (cast `/Game/_Game/Character/BP_BaseCharacter` OtherActor))
  (`KismetArrayLibrary.Array_RemoveItem` (`self.OverlapingActors`) _asbp_base_character))

(fn `UserConstructionScript`)