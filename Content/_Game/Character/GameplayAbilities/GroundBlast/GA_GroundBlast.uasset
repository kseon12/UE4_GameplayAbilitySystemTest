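; Ground Blast gameplay ability: a player-aimed area attack that damages characters and launches them upward with a stun.
; After a cost check and cast montage, it enables camera-controlled rotation and waits for user-confirmed target data from the ground-select target actor.
; Confirmation commits the ability, starts UI cooldown and plays the end-cast montage, spawning the blast effect and applying damage and push.
; Ending the ability cancels targeting and restores rotation.
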(event `self.K2_ActivateAbility`
  (bind _returnvalue (`self.K2_CheckAbilityCost`))
  (if _returnvalue
    (`AbilityTask_PlayMontageAndWait.CreatePlayMontageAndWaitProxy` "None" "/Game/_Game/Character/Animation/AM_Cast_GroundBlast.AM_Cast_GroundBlast"
      (:`then`
        (`KismetSystemLibrary.Delay` (`AnimSequenceBase.SequenceLength` (`self.GetCurrentMontage`)))
        (bind _basecharacter (`self.Get Player Character and Controller`))
        (`/Game/_Game/Character/BP_BaseCharacter.MakeCameraControlRotation` _basecharacter true)
        (bind (_asynctaskproxy _data) (`AbilityTask_WaitTargetData.WaitTargetData` "None" "UserConfirmed" "/Game/_Game/Character/GameplayAbilities/GroundBlast/BP_GATargetActor_GroundSelect.BP_GATargetActor_GroundSelect_C" 200.0 (struct) (struct) null)
          (:`ValidData`
            (bind _basecharacter_2 (`self.Get Player Character and Controller`))
            (set `/Game/_Game/Character/BP_BaseCharacter.bIsTargeting ` false _basecharacter_2)
            (`self.K2_CommitAbility`)
            (`self.DoUICooldown`)
            (`AbilityTask_PlayMontageAndWait.CreatePlayMontageAndWaitProxy` "None" "/Game/_Game/Character/Animation/AM_EndCast_GroundBlast.AM_EndCast_GroundBlast"
              (:`then`
                (`GameplayStatics.SpawnEmitterAtLocation` "/Game/_Game/Character/GameplayAbilities/GroundBlast/P_GroundBlast.P_GroundBlast" (`AbilitySystemBlueprintLibrary.GetTargetDataEndPoint` _data (- (`AbilitySystemBlueprintLibrary.GetDataCountFromTargetData` _data) 1)))
                (`self.BP_ApplyGameplayEffectToTarget` _data "/Game/_Game/Character/GameplayAbilities/GroundBlast/GE_GroundBlast_Damage.GE_GroundBlast_Damage_C")
                (for _array_element (`AbilitySystemBlueprintLibrary.GetActorsFromTargetData` _data)
                  (bind _asbp_base_character (cast `/Game/_Game/Character/BP_BaseCharacter` _array_element))
                  (`/Game/_Game/Character/BP_BaseCharacter.PushCharacter` _asbp_base_character (0.0 0.0 1.0) 1000.0 2.0 "/Game/_Game/Character/Animation/AM_GroundBlastPush.AM_GroundBlastPush")))
              (:`OnCompleted`
                (`self.K2_EndAbility` :!label _label))
              (:`OnBlendOut`
                (goto _label))
              (:`OnInterrupted`
                (goto _label))
              (:`OnCancelled`
                (goto _label))))
          (:`Cancelled`
            (`self.K2_EndAbility`)))))
    (else
      (`self.K2_EndAbility`))))

(event `self.K2_OnEndAbility`
  (params (bWasCancelled :type Boolean))
  (bind _basecharacter (`self.Get Player Character and Controller`))
  (`AbilitySystemComponent.TargetCancel` (`AbilitySystemBlueprintLibrary.GetAbilitySystemComponent` _basecharacter))
  (bind _basecharacter_2 (`self.Get Player Character and Controller`))
  (`/Game/_Game/Character/BP_BaseCharacter.MakeCameraControlRotation` _basecharacter_2 false))