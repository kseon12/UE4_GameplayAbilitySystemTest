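; Gameplay ability for a dash that launches the owning character forward, damaging and knocking back characters hit along the way.
; On activation it commits, starts the UI cooldown, zeroes ground friction, applies a forward impulse and sets pawn collision to overlap.
; While the dash montage plays, a damage gameplay event applies the damage effect and pushes the target away with a stun.
; Ending the ability restores friction and blocking collision.
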(event `self.K2_ActivateAbility`
  (`self.K2_CommitAbility`)
  (`self.DoUICooldown`)
  (bind _ascharacter (cast `Character` (`self.GetOwningActorFromActorInfo`))
    (:`then`
      (bind _charactermovement (`Character.CharacterMovement` _ascharacter))
      (set `self.OriginalGroundFriction` (`CharacterMovementComponent.GroundFriction` _charactermovement))
      (set `CharacterMovementComponent.GroundFriction` 0.0 _charactermovement)
      (`CharacterMovementComponent.AddImpulse` _charactermovement (* (`Actor.GetActorForwardVector` _ascharacter) 2000.0) true)
      (bind _basecharacter (`self.Get Player Character and Controller`))
      (`/Game/_Game/Character/BP_BaseCharacter.SetCollisionToPawn` _basecharacter "ECR_Overlap")
      (`AbilityTask_PlayMontageAndWait.CreatePlayMontageAndWaitProxy` "None" "/Game/_Game/Character/Animation/AM_Cast_Dash.AM_Cast_Dash"
        (:`then`
          (bind (_asynctaskproxy _payload) (`AbilityTask_WaitGameplayEvent.WaitGameplayEvent` (struct :`TagName` "Skill.Dash.DealDamage") null)
            (:`EventReceived`
              (bind (_eventtag _instigator _target) (break `GameplayEventData` _payload))
              (`self.BP_ApplyGameplayEffectToTarget` (`AbilitySystemBlueprintLibrary.AbilityTargetDataFromActor` _target) "/Game/_Game/Character/GameplayAbilities/Dash/GE_Dash_Damage.GE_Dash_Damage_C")
              (bind _asbp_base_character (cast `/Game/_Game/Character/BP_BaseCharacter` _target))
              (`/Game/_Game/Character/BP_BaseCharacter.PushCharacter` _asbp_base_character (`KismetMathLibrary.Normal` (- (`Actor.K2_GetActorLocation` _asbp_base_character) (`Actor.K2_GetActorLocation` (`self.GetOwningActorFromActorInfo`))) 0.0) 2000.0 3.0 null))))
        (:`OnCompleted`
          (`self.K2_EndAbility` :!label _label))
        (:`OnBlendOut`
          (goto _label))
        (:`OnInterrupted`
          (goto _label))
        (:`OnCancelled`
          (goto _label))))
    (:`CastFailed`
      (`self.K2_EndAbility`))))

(event `self.K2_OnEndAbility`
  (params (bWasCancelled :type Boolean))
  (bind _ascharacter (cast `Character` (`self.GetOwningActorFromActorInfo`)))
  (set `CharacterMovementComponent.GroundFriction` (`self.OriginalGroundFriction`) (`Character.CharacterMovement` _ascharacter))
  (bind _basecharacter (`self.Get Player Character and Controller`))
  (`/Game/_Game/Character/BP_BaseCharacter.SetCollisionToPawn` _basecharacter "ECR_Block"))