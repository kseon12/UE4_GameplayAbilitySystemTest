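; BP_FireBall is the fireball actor for a GAS ability, limited to a ten-second lifespan.
; When its sphere overlaps a BP_BaseCharacter, it runs a hostility check between that character and its instigator.
; On a hostile hit, the instigator applies the fireball's stored Gameplay Effect spec handle to the target through actor-based target data, then the fireball destroys itself.
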(event `self.ReceiveBeginPlay`
  (`self.SetLifeSpan` 10.0))

(event `self.Sphere.OnComponentBeginOverlap`
  (params (OverlappedComponent :type "PrimitiveComponent Object Reference") (OtherActor :type "Actor Object Reference") (OtherComp :type "PrimitiveComponent Object Reference") (OtherBodyIndex :type Integer) (bFromSweep :type Boolean) (SweepResult :type "HitResult Structure (by ref)"))
  (bind _asbp_base_character (cast `/Game/_Game/Character/BP_BaseCharacter` OtherActor))
  (bind _asbase_character (cast `BaseCharacter` (`self.GetInstigator`)))
  (bind _returnvalue (`BaseCharacter.IsTargetHostile` _asbp_base_character _asbase_character))
  (if _returnvalue
    (`BaseCharacter.ApplyGESpecHandleToTargetDataSpecHandle` _asbase_character (`self.GESpecHandle`) (`AbilitySystemBlueprintLibrary.AbilityTargetDataFromActor` OtherActor))
    (`self.K2_DestroyActor`)))

(fn `UserConstructionScript`)