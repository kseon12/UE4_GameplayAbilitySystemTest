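; Fire Blast gameplay ability that pulls nearby characters toward the caster, then blasts them away with damage.
; A cast montage drives it through Pull and Push gameplay events, and the ability ends with the montage.
; Pull gathers targets instantly with GATargetActor_Around and drags them in with a stun.
; Push reuses that target data for damage and a stronger stunning shove, taking its direction from the pull loop's character reference.
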(event `self.K2_ActivateAbility`
  (bind _data (`self.Data`))
  (`self.K2_CommitAbility`)
  (`self.DoUICooldown`)
  (`AbilityTask_PlayMontageAndWait.CreatePlayMontageAndWaitProxy` "None" "/Game/_Game/Character/Animation/AM_Cast_FireBlast.AM_Cast_FireBlast"
    (:`then`
      (`AbilityTask_WaitGameplayEvent.WaitGameplayEvent` (struct :`TagName` "Skill.FireBlast.Pull") null
        (:`then`
          (`AbilityTask_WaitGameplayEvent.WaitGameplayEvent` (struct :`TagName` "Skill.FireBlast.Push") null
            (:`EventReceived`
              (`self.BP_ApplyGameplayEffectToTarget` _data "/Game/_Game/Character/GameplayAbilities/FireBlast/GE_FireBlast_Damage.GE_FireBlast_Damage_C")
              (for _array_element (`AbilitySystemBlueprintLibrary.GetActorsFromTargetData` _data)
                (bind _asbp_base_character (cast `/Game/_Game/Character/BP_BaseCharacter` _array_element))
                (bind _returnvalue (`KismetMathLibrary.Normal` (- (`Actor.K2_GetActorLocation` (`self.GetOwningActorFromActorInfo`)) (`Actor.K2_GetActorLocation` (stale _asbp_base_character_2)))))
                (`/Game/_Game/Character/BP_BaseCharacter.PushCharacter` _asbp_base_character (* _returnvalue -1.0) 4000.0 2.0 null)))))
        (:`EventReceived`
          (bind (_asynctaskproxy _data_2) (`AbilityTask_WaitTargetData.WaitTargetData` "None" "Instant" "/Script/GAS_Test.GATargetActor_Around" 400.0 (struct) (struct) null)
            (:`ValidData`
              (set `self.Data` _data_2)
              (for _array_element_2 (`AbilitySystemBlueprintLibrary.GetActorsFromTargetData` _data_2)
                (bind _asbp_base_character_2 (cast `/Game/_Game/Character/BP_BaseCharacter` _array_element_2))
                (`/Game/_Game/Character/BP_BaseCharacter.PushCharacter` _asbp_base_character_2 _returnvalue 1000.0 2.0 null)))))))
    (:`OnCompleted`
      (`self.K2_EndAbility` :!label _label))
    (:`OnBlendOut`
      (goto _label))
    (:`OnInterrupted`
      (goto _label))
    (:`OnCancelled`
      (goto _label))))