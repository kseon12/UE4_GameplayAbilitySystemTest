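; GA_Melee_Combo_03 is a melee attack gameplay ability that plays the AM_Melee_Combo_01 montage, despite its 03 name.
; While the montage runs, it listens for the DealDamage gameplay event and applies GE_Melee_Damage to the payload target.
; Targets that are BP_BaseCharacter are also pushed away from the attacker and briefly stunned.
; The ability ends when the montage completes, blends out, is interrupted or is cancelled.
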(event `self.K2_ActivateAbility`
  (`self.K2_CommitAbility`)
  (`AbilityTask_PlayMontageAndWait.CreatePlayMontageAndWaitProxy` "None" "/Game/_Game/Character/Animation/AM_Melee_Combo_01.AM_Melee_Combo_01"
    (:`then`
      (bind (_asynctaskproxy _payload) (`AbilityTask_WaitGameplayEvent.WaitGameplayEvent` (struct :`TagName` "Abilities.Attack.Melee.DealDamage") null)
        (:`EventReceived`
          (bind (_eventtag _instigator _target) (break `GameplayEventData` _payload))
          (`self.BP_ApplyGameplayEffectToTarget` (`AbilitySystemBlueprintLibrary.AbilityTargetDataFromActor` _target) "/Game/_Game/Character/GameplayAbilities/Melee/GE_Melee_Damage.GE_Melee_Damage_C")
          (bind _asbp_base_character (cast `/Game/_Game/Character/BP_BaseCharacter` _target))
          (`/Game/_Game/Character/BP_BaseCharacter.PushCharacter` _asbp_base_character (`KismetMathLibrary.Normal` (- (`Actor.K2_GetActorLocation` _asbp_base_character) (`Actor.K2_GetActorLocation` (`self.GetOwningActorFromActorInfo`))) 0.0) 200.0 0.3 null))))
    (:`OnCompleted`
      (`self.K2_EndAbility` :!label _label))
    (:`OnBlendOut`
      (goto _label))
    (:`OnInterrupted`
      (goto _label))
    (:`OnCancelled`
      (goto _label))))