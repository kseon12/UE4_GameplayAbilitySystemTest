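; GA_Melee_Combo_01 is a Gameplay Ability for a melee combo attack on BP_BaseCharacter.
; On activation it commits, advances the owner's combo sequence and plays that character's MeleeMontage.
; While the montage plays, it waits for DealDamage gameplay events, applies GE_Melee_Damage at the owner's DamageLevel to the target, and pushes and briefly stuns hit characters away from the attacker.
; The ability ends when the montage completes, blends out or is interrupted or cancelled.
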(event `self.K2_ActivateAbility`
  (`self.K2_CommitAbility`)
  (bind _asbp_base_character (cast `/Game/_Game/Character/BP_BaseCharacter` (`self.GetOwningActorFromActorInfo`)))
  (`/Game/_Game/Character/BP_BaseCharacter.DoComboSequence` _asbp_base_character)
  (`AbilityTask_PlayMontageAndWait.CreatePlayMontageAndWaitProxy` "None" (`/Game/_Game/Character/BP_BaseCharacter.MeleeMontage` _asbp_base_character)
    (:`then`
      (bind (_asynctaskproxy _payload) (`AbilityTask_WaitGameplayEvent.WaitGameplayEvent` (struct :`TagName` "Abilities.Attack.Melee.DealDamage") null)
        (:`EventReceived`
          (bind (_eventtag _instigator _target) (break `GameplayEventData` _payload))
          (`self.BP_ApplyGameplayEffectToTarget` (`AbilitySystemBlueprintLibrary.AbilityTargetDataFromActor` _target) "/Game/_Game/Character/GameplayAbilities/Melee/GE_Melee_Damage.GE_Melee_Damage_C" (`/Game/_Game/Character/BP_BaseCharacter.DamageLevel` _asbp_base_character))
          (bind _asbp_base_character_2 (cast `/Game/_Game/Character/BP_BaseCharacter` _target))
          (`/Game/_Game/Character/BP_BaseCharacter.PushCharacter` _asbp_base_character_2 (`KismetMathLibrary.Normal` (- (`Actor.K2_GetActorLocation` _asbp_base_character_2) (`Actor.K2_GetActorLocation` (`self.GetOwningActorFromActorInfo`))) 0.0) 200.0 0.3 null))))
    (:`OnCompleted`
      (`self.K2_EndAbility` :!label _label))
    (:`OnBlendOut`
      (goto _label))
    (:`OnInterrupted`
      (goto _label))
    (:`OnCancelled`
      (goto _label))))