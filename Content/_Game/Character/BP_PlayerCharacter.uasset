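; Player character Blueprint that shows changes in health, mana and strength on the player's HUD.
; Each change event casts the controller to BP_BasePlayerController and passes the current-to-max ratio to the matching glass bar in its MainWidget.
; If the cast fails, nothing updates; BeginPlay, overlap and Tick are unused placeholders, and the construction script only calls its parent.
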(event `self.BP_OnHealthChanged`
  (params (Health :type "Float (single-precision)") (MaxHealth :type "Float (single-precision)"))
  (bind _asbp_base_player_controller (cast `/Game/_Game/Character/BP_BasePlayerController` (`self.GetController`)))
  (`/Game/_Game/UI/WBP_GlassHealthBar.SetPercentage` (`/Game/_Game/UI/WBP_Main.WBP_GlassHealthBar` (`/Game/_Game/Character/BP_BasePlayerController.MainWidget` _asbp_base_player_controller)) (/ Health MaxHealth)))

(event `self.BP_OnManaChanged`
  (params (Mana :type "Float (single-precision)") (MaxMana :type "Float (single-precision)"))
  (bind _asbp_base_player_controller (cast `/Game/_Game/Character/BP_BasePlayerController` (`self.GetController`)))
  (`/Game/_Game/UI/WBP_GlassManaBar.SetPercentage` (`/Game/_Game/UI/WBP_Main.WBP_GlassManaBar` (`/Game/_Game/Character/BP_BasePlayerController.MainWidget` _asbp_base_player_controller)) (/ Mana MaxMana)))

(event `self.BP_OnStrengthChanged`
  (params (Strength :type "Float (single-precision)") (MaxStrength :type "Float (single-precision)"))
  (bind _asbp_base_player_controller (cast `/Game/_Game/Character/BP_BasePlayerController` (`self.GetController`)))
  (`/Game/_Game/UI/WBP_GlassStrengthBar.SetPercentage` (`/Game/_Game/UI/WBP_Main.WBP_GlassStrengthBar` (`/Game/_Game/Character/BP_BasePlayerController.MainWidget` _asbp_base_player_controller)) (/ Strength MaxStrength)))

(fn `UserConstructionScript`
  (`parent.UserConstructionScript`))