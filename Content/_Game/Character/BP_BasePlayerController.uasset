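; BP_BasePlayerController is a player controller that turns player input into pawn movement, camera look and character abilities.
; Move axes push the controlled pawn along the camera's forward and right vectors, while look axes add pitch and yaw.
; Jump, melee attack, health regen and dash presses cast the pawn to BP_BaseCharacter and call its matching function.
; On BeginPlay it creates the WBP_Main widget, stores it and adds it to the viewport.
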(event `InputAxis|MoveForward`
  (params (AxisValue :type "Float (single-precision)"))
  ;[1 1 1] Comment
  (`Pawn.AddMovementInput` (`self.K2_GetPawn`) (`KismetMathLibrary.GetForwardVector` (`PlayerCameraManager.GetCameraRotation` (`self.PlayerCameraManager`))) AxisValue false))

(event `InputAction|Jump`
  (params (Key :type "Key Structure"))
  ;[1 1 1] Comment
  (:`Pressed`
    (bind _asbp_base_character (cast `/Game/_Game/Character/BP_BaseCharacter` (`self.K2_GetPawn`)))
    (`Character.Jump` _asbp_base_character)))

(event `InputAxis|LookUp`
  (params (AxisValue :type "Float (single-precision)"))
  ;[1 1 1] Comment
  (`self.AddPitchInput` AxisValue))

(event `InputAxis|MoveRight`
  (params (AxisValue :type "Float (single-precision)"))
  ;[1 1 1] Comment
  (`Pawn.AddMovementInput` (`self.K2_GetPawn`) (`KismetMathLibrary.GetRightVector` (`PlayerCameraManager.GetCameraRotation` (`self.PlayerCameraManager`))) AxisValue false))

(event `InputAxis|Turn`
  (params (AxisValue :type "Float (single-precision)"))
  ;[1 1 1] Comment
  (`self.AddYawInput` AxisValue))

(event `InputAction|Attack`
  (params (Key :type "Key Structure"))
  ;[1 1 1] Comment
  (:`Pressed`
    (bind _asbp_base_character (cast `/Game/_Game/Character/BP_BaseCharacter` (`self.K2_GetPawn`)))
    (`/Game/_Game/Character/BP_BaseCharacter.MeleeAtack` _asbp_base_character)))

(event `self.ReceiveBeginPlay`
  (bind _returnvalue (`|CreateWidget` "/Game/_Game/UI/WBP_Main.WBP_Main_C"))
  (bind _output_get (set `self.MainWidget` _returnvalue))
  (`UserWidget.AddToViewport` _output_get 0))

(event `InputAction|HealthRegen`
  (params (Key :type "Key Structure"))
  ;[1 1 1] Comment
  (:`Pressed`
    (bind _asbp_base_character (cast `/Game/_Game/Character/BP_BaseCharacter` (`self.K2_GetPawn`)))
    (`/Game/_Game/Character/BP_BaseCharacter.TryHealthRegen` _asbp_base_character)))

(event `InputAction|Dash`
  (params (Key :type "Key Structure"))
  ;[1 1 1] Comment
  (:`Pressed`
    (bind _asbp_base_character (cast `/Game/_Game/Character/BP_BaseCharacter` (`self.K2_GetPawn`)))
    (`/Game/_Game/Character/BP_BaseCharacter.TryDash` _asbp_base_character)))

(fn `UserConstructionScript`)