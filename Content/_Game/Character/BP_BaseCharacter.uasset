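; Base GAS character providing melee combos, hit detection, knockback and death, granting initial abilities and a regen effect on BeginPlay.
; Melee input confirms targeting or activates the combo ability, while DoComboSequence cycles three montages with matching damage levels.
; Sword and capsule overlaps with hostile characters send melee and dash damage gameplay events to itself.
; PushCharacter launches by impulse, temporarily zeroing friction and ignoring pawn collision, with optional stun and combo reset.
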(event `self.ReceiveBeginPlay`
  (`self.AddAbilities` (`self.InittialAbilities`))
  (`AbilitySystemComponent.BP_ApplyGameplayEffectToSelf` :`self` (`self.AbilitySystemComponent`) :`GameplayEffectClass` "/Game/_Game/Character/GameplayAbilities/General/GE_BasicRegen.GE_BasicRegen_C"))

(event `MeleeAtack`
  ;[1 1 1] Comment
  (if (`self.bIsTargeting `)
    (`AbilitySystemComponent.TargetConfirm` (`self.AbilitySystemComponent`))
    (else
      (`AbilitySystemComponent.TryActivateAbilityByClass` (`self.AbilitySystemComponent`) "/Game/_Game/Character/GameplayAbilities/Melee/GA_Melee_Combo_01.GA_Melee_Combo_01_C" true))))

(event `self.SwordCapsuleComponent.OnComponentBeginOverlap`
  (params (OverlappedComponent :type "PrimitiveComponent Object Reference") (OtherActor :type "Actor Object Reference") (OtherComp :type "PrimitiveComponent Object Reference") (OtherBodyIndex :type Integer) (bFromSweep :type Boolean) (SweepResult :type "HitResult Structure (by ref)"))
  ;[1 1 1] Comment
  (bind _asbp_base_character (cast `/Game/_Game/Character/BP_BaseCharacter` OtherActor))
  (bind _returnvalue (`self.IsTargetHostile` _asbp_base_character self))
  (if _returnvalue
    (`AbilitySystemBlueprintLibrary.SendGameplayEventToActor` self (struct :`TagName` "Abilities.Attack.Melee.DealDamage") (make `GameplayEventData` (struct) null OtherActor))))

(event `self.BP_Die`
  ;[1 1 1] Comment
  (bind _returnvalue (`self.PlayAnimMontage` "/Game/_Game/Character/Animation/AM_Death.AM_Death"))
  (`KismetSystemLibrary.Delay` _returnvalue)
  (`self.K2_DestroyActor`))

(event `self.CapsuleComponent.OnComponentBeginOverlap`
  (params (OverlappedComponent :type "PrimitiveComponent Object Reference") (OtherActor :type "Actor Object Reference") (OtherComp :type "PrimitiveComponent Object Reference") (OtherBodyIndex :type Integer) (bFromSweep :type Boolean) (SweepResult :type "HitResult Structure (by ref)"))
  ;[1 1 1] Comment
  (bind _asbp_base_character (cast `/Game/_Game/Character/BP_BaseCharacter` OtherActor))
  (if (not (`KismetArrayLibrary.Array_Contains` (`self.OverlapActorArray`) _asbp_base_character))
    (`KismetArrayLibrary.Array_AddUnique` (`self.OverlapActorArray`) _asbp_base_character)
    (bind _returnvalue (`self.IsTargetHostile` self _asbp_base_character))
    (if _returnvalue
      (`AbilitySystemBlueprintLibrary.SendGameplayEventToActor` self (struct :`TagName` "Skill.Dash.DealDamage") (make `GameplayEventData` (struct) self OtherActor)))))

(event `PushCharacter`
  (params (ImpulsDirection :type "Vector Structure") (PushStrength :type "Float (double-precision)") (StunDuration :type "Float (double-precision)") (AnimMontage :type "AnimMontage Object Reference"))
  (bind _groundfriction (`CharacterMovementComponent.GroundFriction` (`self.CharacterMovement`)))
  ;[1 1 1] Comment
  (`self.SetCollisionToPawn` "ECR_Ignore")
  (`self.PlayAnimMontage` AnimMontage)
  (if (> _groundfriction 0.0)
    (set `self.PreviousGroundFriction` _groundfriction))
  (`self.SetGroundFriction` 0.0)
  (`CharacterMovementComponent.AddImpulse` (`self.CharacterMovement`) (* ImpulsDirection PushStrength) true)
  (if (> StunDuration 0.0)
    (`self.HitStun` StunDuration))
  (`KismetSystemLibrary.Delay` 0.5)
  (`self.SetGroundFriction` (`self.PreviousGroundFriction`))
  (`self.SetCollisionToPawn` "ECR_Block")
  (set `self.ComboCount` 0))

(event `MakeCameraControlRotation`
  (params (ShouldControlRotation :type Boolean))
  ;[1 1 1] Comment
  (if ShouldControlRotation
    (set `self.bUseControllerRotationYaw` true)
    (set `CharacterMovementComponent.bOrientRotationToMovement` false (`self.CharacterMovement`))
    (else
      (set `self.bUseControllerRotationYaw` false)
      (set `CharacterMovementComponent.bOrientRotationToMovement` true (`self.CharacterMovement`)))))

(fn `DoComboSequence`
  (switch `int` (`self.ComboCount`)
    (:`0`
      (set `self.MeleeMontage` "/Game/_Game/Character/Animation/AM_Melee_Combo_01.AM_Melee_Combo_01")
      (`/Engine/EditorBlueprintResources/StandardMacros.IncrementInt` (`self.ComboCount`)
        (:`  `
          (set `self.DamageLevel` 1))))
    (:`1`
      (set `self.MeleeMontage` "/Game/_Game/Character/Animation/AM_Melee_Combo_02.AM_Melee_Combo_02")
      (`/Engine/EditorBlueprintResources/StandardMacros.IncrementInt` (`self.ComboCount`)
        (:`  `
          (set `self.DamageLevel` 2))))
    (:`2`
      (set `self.MeleeMontage` "/Game/_Game/Character/Animation/AM_Melee_Combo_03.AM_Melee_Combo_03")
      (set `self.ComboCount` 0)
      (set `self.DamageLevel` 3))))

(fn `SetCollisionToPawn`
  (params (CollisionResponse :type "ECollisionResponse Enum" :default "ECR_Overlap"))
  (`PrimitiveComponent.SetCollisionResponseToChannel` (`self.CapsuleComponent`) "ECC_Pawn" CollisionResponse))

(fn `SetGroundFriction`
  (params (Value :type "Float (double-precision)"))
  (set `CharacterMovementComponent.GroundFriction` Value (`self.CharacterMovement`)))

(fn `UserConstructionScript`)